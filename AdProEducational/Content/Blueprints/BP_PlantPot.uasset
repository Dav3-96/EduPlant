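; BP_PlantPot is a plant pot that spawns an actor of the PlantToSpawn class at its PlantLoc component's transform.
; On BeginPlay it spawns the plant if AlreadyCreated is set, and otherwise the Plant event can spawn it through a DoOnce gate fed by that flag.
; Both paths store the spawned actor and copy its InfoText onto the pot.
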(event Custom|Plant
  (params (UI :type In%20Game%20UI%20Object%20Reference))
  (Utilities|FlowControl|DoOnce (Variables|Default|GetAlreadyCreated?)
    (:Completed
      (bind _returnvalue (Game|SpawnActorfromClass (Variables|Default|GetPlantToSpawn) (Transformation|GetWorldTransform (Variables|Default|GetPlantLoc)) "Undefined" 0 0))
      (bind _output_get (Variables|Default|SetSpawnedActor _returnvalue))
      (Variables|Default|SetInfo%20Text (Variables|/Game/Blueprints/BP_Plant.BP_Plant_C|GetInfoText _output_get)))))

(event EventBeginPlay
  (if (Variables|Default|GetAlreadyCreated?)
    (bind _returnvalue (Game|SpawnActorfromClass (Variables|Default|GetPlantToSpawn) (Transformation|GetWorldTransform (Variables|Default|GetPlantLoc)) "Undefined" 0 0))
    (bind _output_get (Variables|Default|SetSpawnedActor _returnvalue))
    (Variables|Default|SetInfo%20Text (Variables|/Game/Blueprints/BP_Plant.BP_Plant_C|GetInfoText _output_get))))

(fn ConstructionScript)